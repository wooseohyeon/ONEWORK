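; BP_Chr is a player character Blueprint that handles movement, look, jump and sprint through Enhanced Input.
; On possession by a PlayerController it adds its input mapping context.
; Move input follows the control rotation's yaw only, and look input drives controller yaw and pitch, with pitch input clamped per event.
; Sprint works by changing SprintRatio, which scales movement input to full while held and half on release or cancel.
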(event `self.ReceivePossessed`
  (params (NewController :type "Controller Object Reference"))
  (bind `_as플레이어_컨트롤러` (cast `PlayerController` NewController))
  (`EnhancedInputSubsystemInterface.AddMappingContext` (pcsubsystem `EnhancedInputLocalPlayerSubsystem` `_as플레이어_컨트롤러`) "/Game/Blueprints/input/NewInputMappingContext.NewInputMappingContext" 0 (struct)))

(event `EnhancedInput|/Game/Blueprints/input/IA_Move`
  (params (ActionValue :type "Vector2D Structure") (ElapsedSeconds :type "Float (double-precision)") (TriggeredSeconds :type "Float (double-precision)") (InputAction :type "InputAction Object Reference" :default "/Game/Blueprints/input/IA_Move.IA_Move"))
  (bind (_returnvalue_roll _returnvalue_pitch _returnvalue_yaw) (`KismetMathLibrary.BreakRotator` (`self.GetControlRotation`)))
  (bind (_returnvalue_roll_2 _returnvalue_pitch_2 _returnvalue_yaw_2) (`KismetMathLibrary.BreakRotator` (`self.GetControlRotation`)))
  (:`Triggered`
    (`self.AddMovementInput` (`KismetMathLibrary.GetForwardVector` (`KismetMathLibrary.MakeRotator` 0.0 0.0 _returnvalue_yaw_2)) (* ActionValue_X (`self.Sprint Ratio`)))
    (`self.AddMovementInput` (`KismetMathLibrary.GetRightVector` (`KismetMathLibrary.MakeRotator` 0.0 0.0 _returnvalue_yaw)) (* ActionValue_Y (`self.Sprint Ratio`)))))

(event `EnhancedInput|/Game/Blueprints/input/IA_Look`
  (params (ActionValue :type "Vector2D Structure") (ElapsedSeconds :type "Float (double-precision)") (TriggeredSeconds :type "Float (double-precision)") (InputAction :type "InputAction Object Reference" :default "/Game/Blueprints/input/IA_Look.IA_Look"))
  (:`Triggered`
    (`self.AddControllerYawInput` ActionValue_X)
    (`self.AddControllerPitchInput` (`KismetMathLibrary.FClamp` ActionValue_Y -0.8 0.8))))

(event `EnhancedInput|/Game/Blueprints/input/IA_Jump`
  (params (ActionValue :type Boolean) (ElapsedSeconds :type "Float (double-precision)") (TriggeredSeconds :type "Float (double-precision)") (InputAction :type "InputAction Object Reference" :default "/Game/Blueprints/input/IA_Jump.IA_Jump"))
  (:`Triggered`
    (if ActionValue
      (`self.Jump`))))

(event `EnhancedInput|/Game/Blueprints/input/IA_Sprint`
  (params (ActionValue :type Boolean) (ElapsedSeconds :type "Float (double-precision)") (TriggeredSeconds :type "Float (double-precision)") (InputAction :type "InputAction Object Reference" :default "/Game/Blueprints/input/IA_Sprint.IA_Sprint"))
  (:`Triggered`
    (set `self.Sprint Ratio` 1.0))
  (:`Canceled`
    (set `self.Sprint Ratio` 0.5 :!label _label))
  (:`Completed`
    (goto _label)))

(fn `UserConstructionScript`)